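; Interactable light switch actor that toggles a linked light on or off when the player interacts with it.
; On Interact, it checks that the Light reference is valid, then reads its LightComponent's current visibility and sets the opposite, without propagating to children.
; The target light is assigned per instance in the Details panel, and BeginPlay, overlap and Tick are unused.
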(event `/Game/Blueprints/Interfaces/BPI_Interaction.Interact`
  (bind _light (`self.Light`))
  (bind _lightcomponent (`Light.LightComponent` _light))
  ;[1 1 1] Light Switch sets visibility of light (declared in details) on and off according to current visibility.
  (`/Engine/EditorBlueprintResources/StandardMacros.IsValid` _light
    (:`Is Valid`
      (if (`SceneComponent.bVisible` _lightcomponent)
        (`SceneComponent.SetVisibility` _lightcomponent false false)
        (else
          (`SceneComponent.SetVisibility` _lightcomponent true false))))))

(fn `UserConstructionScript`
  (`parent.UserConstructionScript`))